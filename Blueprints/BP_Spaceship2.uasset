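; BP_Spaceship2 is a player-controlled, physics-driven spaceship with toggleable cockpit and external cameras.
; Roll, pitch and yaw axes each drive a pair of thruster components at opposite ends of the ship, scaled by input and deactivated at zero.
; EngineThrust and SpeedUp add impulses to the mesh along the root arrow's forward vector, without delta-time scaling.
; It also exposes its chat component and the PlayerState name through getters.
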(event Input|ActionEvents|InputActionToggleCameraView
  (params (Key :type Key%20Structure))
  (bind _cockpitcamera (Variables|Default|GetCockpitCamera))
  (bind _externalcamera (Variables|Default|GetExternalCamera))
  ;[1 1 1] Switch camera
  (:Pressed
    (Utilities|FlowControl|FlipFlop
      (:A
        (Components|Activation|Activate _cockpitcamera false)
        (Components|Activation|Deactivate _externalcamera))
      (:B
        (Components|Activation|Activate _externalcamera false)
        (Components|Activation|Deactivate _cockpitcamera)))))

(event Input|AxisEvents|InputAxisSpeedUp
  (params (AxisValue :type Float%20%28single-precision%29))
  (Physics|AddImpulse (Variables|Default|GetShipMesh) (* (Math|Vector|GetForwardVector (Transformation|GetWorldRotation (Variables|Default|GetRootDirectionArrow))) (* AxisValue (Variables|Default|GetSpeedUpPower))) "None" false))

(event Input|AxisEvents|InputAxisYaw
  (params (AxisValue :type Float%20%28single-precision%29))
  (bind _yawstrength (Variables|Default|GetYawStrength))
  (bind _noseyawthrust (Variables|Default|GetNoseYawThrust))
  (bind _tailyawthrust (Variables|Default|GetTailYawThrust))
  (bind _returnvalue (* AxisValue _yawstrength))
  ;[1 1 1] Handless Yawing
  (if (!= AxisValue 0.0)
    (Variables|/Script/Engine.PhysicsThrusterComponent|SetThrustStrength _noseyawthrust _returnvalue)
    (Variables|/Script/Engine.PhysicsThrusterComponent|SetThrustStrength _tailyawthrust _returnvalue)
    (Components|Activation|Activate _noseyawthrust false)
    (Components|Activation|Activate _tailyawthrust false)
    (else
      (Components|Activation|Deactivate (Variables|Default|GetNoseYawThrust))
      (Components|Activation|Deactivate (Variables|Default|GetTailYawThrust)))))

(event Input|AxisEvents|InputAxisEngineThrust
  (params (AxisValue :type Float%20%28single-precision%29))
  (Physics|AddImpulse (Variables|Default|GetShipMesh) (* (Math|Vector|GetForwardVector (Transformation|GetWorldRotation (Variables|Default|GetRootDirectionArrow))) (* AxisValue (Variables|Default|GetEnginePower))) "None" false))

(event Input|AxisEvents|InputAxisRoll
  (params (AxisValue :type Float%20%28single-precision%29))
  (bind _rollstrength (Variables|Default|GetRollStrength))
  (bind _leftwingrollthrust (Variables|Default|GetLeftWingRollThrust))
  (bind _rightwingrollthrust (Variables|Default|GetRightWingRollThrust))
  (bind _returnvalue (* AxisValue _rollstrength))
  ;[1 1 1] Handless Rolling
  (if (!= AxisValue 0.0)
    (Variables|/Script/Engine.PhysicsThrusterComponent|SetThrustStrength _leftwingrollthrust _returnvalue)
    (Variables|/Script/Engine.PhysicsThrusterComponent|SetThrustStrength _rightwingrollthrust _returnvalue)
    (Components|Activation|Activate _leftwingrollthrust false)
    (Components|Activation|Activate _rightwingrollthrust false)
    (else
      (Components|Activation|Deactivate (Variables|Default|GetLeftWingRollThrust))
      (Components|Activation|Deactivate (Variables|Default|GetRightWingRollThrust)))))

(event Input|AxisEvents|InputAxisPitch
  (params (AxisValue :type Float%20%28single-precision%29))
  (bind _pitchstrength (Variables|Default|GetPitchStrength))
  (bind _nosepitchthrust (Variables|Default|GetNosePitchThrust))
  (bind _tailpitchthrust (Variables|Default|GetTailPitchThrust))
  (bind _returnvalue (* AxisValue _pitchstrength))
  ;[1 1 1] Handless Pitching
  (if (!= AxisValue 0.0)
    (Variables|/Script/Engine.PhysicsThrusterComponent|SetThrustStrength _nosepitchthrust _returnvalue)
    (Variables|/Script/Engine.PhysicsThrusterComponent|SetThrustStrength _tailpitchthrust _returnvalue)
    (Components|Activation|Activate _nosepitchthrust false)
    (Components|Activation|Activate _tailpitchthrust false)
    (else
      (Components|Activation|Deactivate (Variables|Default|GetNosePitchThrust))
      (Components|Activation|Deactivate (Variables|Default|GetTailPitchThrust)))))

(fn ConstructionScript)

(fn GetChatComponent
  (return (Variables|Default|GetSimpleChat_Comp)))

(fn GetPlayerName
  (return (PlayerState|GetPlayerName (Variables|GetPlayerState))))